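; Base character Blueprint that equips a fruit cannon and handles feedback for damage, score, powerups, stun and death.
; Health component damage events drive floating numbers, tinted while shielded, and controller rumble; player state score increases spawn player-colored totals.
; Tick toggles foot dust by velocity and syncs the shield effect on a shared powerup particle system.
; Death ragdolls the mesh, hides the HUD, disables input and clears the outline.
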(event Custom|ActivateRFX
  (params (RFXSystem :type Niagara%20System%20Object%20Reference) (TimeActive :type Float%20%28single-precision%29) (DeactivateSelf :type Boolean))
  (bind _fxe_powerup_system (Variables|Default|GetFXE_Powerup_System))
  ;[1 1 1] Activate and deactivate powerup effects
  (if (not (Components|Activation|IsActive (Variables|Default|GetFXE_Powerup_System)))
    (Class|NiagaraComponent|SetAsset _fxe_powerup_system RFXSystem true)
    (Components|Activation|Activate _fxe_powerup_system false)
    (if DeactivateSelf
      (Utilities|FlowControl|Delay TimeActive)
      (Components|Activation|Deactivate _fxe_powerup_system))))

(event Custom|Rumble%20Controller
  (params (DamageAmount :type Float%20%28single-precision%29) (Source :type Controller%20Object%20Reference))
  (bind _playercontroller (Variables|Default|GetplayerController))
  ;[1 1 1] controller rumble
  (Utilities|IsValid _playercontroller
    (:Is%20Valid
      (Game|Feedback|PlayDynamicForceFeedback _playercontroller (Math|Float|Clamp(Float) (/ DamageAmount 5e+01) 0.0 0.35) 0.25 true true true true))))

(event Custom|Show%20Score%20Increase
  (params (scoreAmount :type Integer))
  (Variables|Default|SetincreasedScore (+ (Variables|Default|GetincreasedScore) scoreAmount))
  (Utilities|FlowControl|Delay 0.1)
  (bind _returnvalue (Game|SpawnActorfromClass "/Game/Blueprints/LevelMechanics/BP_env_FloatingText.BP_env_FloatingText_C" (Math|Conversions|ToTransform(Vector) (Transformation|GetActorLocation)) "Undefined" 0 0))
  (Default|Initialize _returnvalue 1.0 (Utilities|Text|ToText(Integer) (Variables|Default|GetincreasedScore)) (Variables|/Script/FruutWars.FWPlayerState|GetPlayerColor (Variables|Default|GetFWPlayerState)))
  (bind _aswbp_floating_text (Utilities|Casting|CastToWBP_FloatingText (UserInterface|GetWidget (Variables|/Game/Blueprints/LevelMechanics/BP_env_FloatingText.BP_env_FloatingText_C|GetText _returnvalue))))
  (Default|SetSize _aswbp_floating_text 40))

(event Custom|Show%20Text
  (params (DamageAmount :type Float%20%28single-precision%29) (Source :type Controller%20Object%20Reference))
  (bind _returnvalue (Utilities|Text|ToText(Float) DamageAmount "HalfToEven" false true 1 324 0 0))
  ;[1 1 1] Hitsplash
  (bind _returnvalue_2 (Game|SpawnActorfromClass "/Game/Blueprints/LevelMechanics/BP_env_FloatingText.BP_env_FloatingText_C" (Math|Conversions|ToTransform(Vector) (Transformation|GetActorLocation)) "Undefined" 0 0))
  (if (> (Variables|/Script/FruutWars.HealthComponent|GetCurrentShield (Variables|Default|GetHealthComponent)) 0.0)
    (Default|Initialize _returnvalue_2 0.5 _returnvalue "(R=0.000000,G=0.509804,B=1.000000,A=1.000000)")
    (else
      (Default|Initialize _returnvalue_2 0.5 _returnvalue "(R=1.000000,G=1.000000,B=1.000000,A=1.000000)"))))

(event Custom|ActivateStunEffect
  (params (Duration :type Float%20%28single-precision%29))
  (bind _returnvalue (Niagara|SpawnSystematLocation "/Game/RFX/System/FXS_StunnedEffect.FXS_StunnedEffect" (Transformation|GetWorldLocation (Variables|Default|GetEffectPos)) "0, 0, 0" "1.000000,1.000000,1.000000" false))
  (Utilities|FlowControl|Delay Duration)
  (Components|DestroyComponent _returnvalue))

(event Custom|Remove%20outline
  ;[1 1 1] remove outline on death
  (Rendering|SetCustomDepthStencilValue (Variables|Character|GetMesh) 0))

(event EventTick
  (params (DeltaSeconds :type Float%20%28single-precision%29))
  (bind _playercontroller (Variables|Default|GetplayerController))
  (bind _fxe_dustyfeet_system (Variables|Default|GetFXE_DustyFeet_System))
  (Utilities|FlowControl|Sequence
    (:then_0
      (if (> (Math|Vector|VectorLengthSquared (Variables|/Script/Engine.MovementComponent|GetVelocity (Pawn|GetMovementComponent))) 0.0)
        (Components|Activation|Activate _fxe_dustyfeet_system false)
        (else
          (Components|Activation|Deactivate _fxe_dustyfeet_system))))
    (:then_1
      ;[1 1 1] Spawn shield if shield rfx was not active
      (if (not (Components|Activation|IsActive (Variables|Default|GetFXE_Powerup_System)))
        (if (> (Variables|/Script/FruutWars.HealthComponent|GetCurrentShield (Variables|Default|GetHealthComponent)) 0.0)
          (CallFunction|ActivateRFX "/Game/RFX/System/FXS_ActivePowerup_Shield.FXS_ActivePowerup_Shield" 0.0 false)
          (Variables|Default|SetHasShields true))))
    (:then_2
      ;[1 1 1] Deactivate shield if you are out of shield
      (if (Variables|Default|GetHasShields)
        (if (Components|Activation|IsActive (Variables|Default|GetFXE_Powerup_System))
          (if (<= (Variables|/Script/FruutWars.HealthComponent|GetCurrentShield (Variables|Default|GetHealthComponent)) 0.0)
            (Components|Activation|Deactivate (Variables|Default|GetFXE_Powerup_System))
            (Variables|Default|SetHasShields false)))))
    (:then_3
      ;[1 1 1] controller rumble
      (Utilities|IsValid _playercontroller
        (:Is%20Valid
          (Game|Feedback|PlayDynamicForceFeedback _playercontroller (Math|Float|Clamp(Float) (/ (stale Custom|Rumble%20Controller DamageAmount) 5e+01) 0.0 0.35) 0.25 true true true true) ; enters at Update
        )))))

(event EventOnCharacterDeath
  (Physics|SetSimulatePhysics (Variables|Character|GetMesh) true)
  (Collision|SetCollisionEnabled (Variables|Default|GetCapsuleComponent) "NoCollision")
  (Collision|SetCollisionEnabled (Variables|Character|GetMesh) "PhysicsOnly")
  (Rendering|SetVisibility (Variables|Default|GetInGameHud) false true)
  (Rendering|SetVisibility (Variables|Default|GetFXE_DustyFeet_System) false false)
  (bind _ascharacter_controller (Utilities|Casting|CastToCharacterController (Pawn|GetController)))
  (Class|CharacterController|DisablePlayerInput _ascharacter_controller))

(event EventBeginPlay
  ;[1 1 1] Spawn primary weapon
  (bind _returnvalue (Game|SpawnActorfromClass "/Game/Blueprints/Weapons/BP_weapon_FruutCannon.BP_weapon_FruutCannon_C" (Math|Transform|MakeTransform "0, 0, 0" "0, 0, 0" "1,1,1") "Undefined" 0 0))
  (Class|BaseCharacter|SetPrimaryWeapon _returnvalue)
  (Collision|SetCollisionEnabled (Variables|Character|GetMesh) "NoCollision")
  (bind _aswbp_ingame_hud (Utilities|Casting|CastToWBP_ingame_Hud (UserInterface|GetWidget (Variables|Default|GetInGameHud))))
  (Variables|/Game/UI/WBP_ingame_Hud.WBP_ingame_Hud_C|SetActiveCharacter _aswbp_ingame_hud self)
  (EventDispatchers|BindEventtoOnDamage (Variables|Default|GetHealthComponent) (delegate Custom|Rumble%20Controller))
  (EventDispatchers|BindEventtoOnDamage (Variables|Default|GetHealthComponent) (delegate Custom|Show%20Text))
  (EventDispatchers|BindEventtoOnDeath (Variables|Default|GetHealthComponent) (delegate Custom|Remove%20outline))
  (Utilities|FlowControl|Sequence
    (:then_0
      (Utilities|FlowControl|Delay 0.2)
      (bind _asfwplayer_state (Utilities|Casting|CastToFWPlayerState (Variables|Default|GetPlayerState)))
      (bind _output_get (Variables|Default|SetFWPlayerState _asfwplayer_state))
      (EventDispatchers|BindEventtoOnScoreIncrease _output_get (delegate Custom|Show%20Score%20Increase)))
    (:then_1
      (bind _asplayer_controller (Utilities|Casting|CastToPlayerController (Pawn|GetController)))
      (Variables|Default|SetplayerController _asplayer_controller))))

(fn ConstructionScript)