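; Commissioner Potato character Blueprint that adds a timed rainbow material effect to show invincibility.
; On first use, it creates dynamic material instances for the mesh's first two material slots and caches them.
; SetRainbowEffect switches their RainbowEffect scalar parameter on, waits for the given duration, then switches it off.
; The Blueprint handles only the visual, with BeginPlay deferring to the parent class.
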(event Custom|SetRainbowEffect
  (params (TimeActive :type Float%20%28single-precision%29))
  ;[1 1 1] Rainbow effect when invicible
  (if (Variables|Default|GetInitRainbow)
    _
    (else
      (CallFunction|InitRainbowEffect)))
  (Rendering|Material|SetScalarParameterValue (Variables|Material|GetM1) "RainbowEffect" 1.0 :!class /Script/Engine.MaterialInstanceDynamic)
  (Rendering|Material|SetScalarParameterValue (Variables|Material|GetM2) "RainbowEffect" 1.0 :!class /Script/Engine.MaterialInstanceDynamic)
  (Utilities|FlowControl|Delay TimeActive)
  ;[1 1 1] Deactivate invincibilty effect
  (Rendering|Material|SetScalarParameterValue (Variables|Material|GetM1) "RainbowEffect" 0.0 :!class /Script/Engine.MaterialInstanceDynamic)
  (Rendering|Material|SetScalarParameterValue (Variables|Material|GetM2) "RainbowEffect" 0.0 :!class /Script/Engine.MaterialInstanceDynamic))

(event Custom|InitRainbowEffect
  (bind _mesh (Variables|Character|GetMesh))
  (bind _returnvalue (Rendering|Material|GetMaterials _mesh))
  (bind _returnvalue_2 (Rendering|Material|CreateDynamicMaterialInstance _mesh 0 (Utilities|Array|Get(acopy) _returnvalue) "None" :!class /Script/Engine.PrimitiveComponent))
  (Variables|Material|SetM1 _returnvalue_2)
  (bind _returnvalue_3 (Rendering|Material|CreateDynamicMaterialInstance _mesh 1 (Utilities|Array|Get(acopy) _returnvalue 1) "None" :!class /Script/Engine.PrimitiveComponent))
  (Variables|Material|SetM2 _returnvalue_3)
  (Rendering|Material|SetMaterial (Variables|Character|GetMesh) 0 (Variables|Material|GetM1))
  (Rendering|Material|SetMaterial (Variables|Character|GetMesh) 1 (Variables|Material|GetM2))
  (Variables|Default|SetInitRainbow true))

(event EventBeginPlay
  (|CallParentFunction))

(fn ConstructionScript)