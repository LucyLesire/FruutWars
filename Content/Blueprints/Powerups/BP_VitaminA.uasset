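; Vitamin A powerup that makes the character who activates it invulnerable through their HealthComponent.
; For BP_cha_CommisionerPotato characters only, it then starts a rainbow effect lasting the component's max invulnerability time and plays a pitch-randomized pickup sound at its own location.
; A SetDamageMultiplier helper sets a valid weapon's damage multiplier but is not called in this graph.
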(event EventBeginPlay)

(event Collision|EventActorBeginOverlap
  (params (OtherActor :type Actor%20Object%20Reference)))

(event EventTick
  (params (DeltaSeconds :type Float%20%28single-precision%29)))

(event EventActivatePowerup
  (params (character :type Base%20Character%20Object%20Reference))
  (bind _healthcomponent (Variables|/Script/FruutWars.BaseCharacter|GetHealthComponent character))
  (Class|HealthComponent|SetInvurnability _healthcomponent true)
  (bind _asbp_cha_commisioner_potato (Utilities|Casting|CastToBP_cha_CommisionerPotato character))
  (Default|SetRainbowEffect _asbp_cha_commisioner_potato (Variables|/Script/FruutWars.HealthComponent|GetMaxInvurnabilityTime _healthcomponent))
  (Audio|PlaySoundatLocation "/Game/Audio/SFX_GetItem.SFX_GetItem" (Transformation|GetActorLocation) "0, 0, 0" 1.0 (Math|Random|RandomFloatinRange 0.9 1.1) 0.0 0 0 0))

(fn ConstructionScript)

(fn SetDamageMultiplier
  (params (Weapon :type Base%20Weapon%20Object%20Reference) (Amount :type Float%20%28single-precision%29))
  (Utilities|IsValid Weapon
    (:Is%20Valid
      (Class|BaseWeapon|SetDamageMultiplier Weapon Amount))))