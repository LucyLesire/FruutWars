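; BP_VitaminE is a damage-boost powerup that doubles weapon damage for the character who activates it.
; On activation it sets the damage multiplier on the primary and, if valid, secondary weapon through a null-checked helper.
; It then shows a self-deactivating damage effect on BP_cha_BaseChar, timed by the primary weapon's max multiplier time.
; A pickup sound plays at its location with randomized pitch.
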(event EventBeginPlay)

(event Collision|EventActorBeginOverlap
  (params (OtherActor :type Actor%20Object%20Reference)))

(event EventTick
  (params (DeltaSeconds :type Float%20%28single-precision%29)))

(event EventActivatePowerup
  (params (character :type Base%20Character%20Object%20Reference))
  (bind _primaryweapon (Variables|/Script/FruutWars.BaseCharacter|GetPrimaryWeapon character))
  (bind _secondaryweapon (Variables|/Script/FruutWars.BaseCharacter|GetSecondaryWeapon character))
  (Utilities|FlowControl|Sequence
    (:then_0
      (CallFunction|SetDamageMultiplier _primaryweapon 2.0)
      (Utilities|IsValid _secondaryweapon
        (:Is%20Valid
          (CallFunction|SetDamageMultiplier _secondaryweapon 2.0))
        (:Is%20Not%20Valid
          _))
      (bind _asbp_cha_base_char (Utilities|Casting|CastToBP_cha_BaseChar character))
      (Default|ActivateRFX _asbp_cha_base_char "/Game/RFX/System/FXS_ActivePowerup_Damage.FXS_ActivePowerup_Damage" (Variables|/Script/FruutWars.BaseWeapon|GetMaxMultiplierTime _primaryweapon) true))
    (:then_1
      (Audio|PlaySoundatLocation "/Game/Audio/SFX_GetItem.SFX_GetItem" (Transformation|GetActorLocation) "0, 0, 0" 1.0 (Math|Random|RandomFloatinRange 0.9 1.1) 0.0 0 0 0))))

(fn ConstructionScript)

(fn SetDamageMultiplier
  (params (Weapon :type Base%20Weapon%20Object%20Reference) (Amount :type Float%20%28single-precision%29))
  (Utilities|IsValid Weapon
    (:Is%20Valid
      (Class|BaseWeapon|SetDamageMultiplier Weapon Amount))))