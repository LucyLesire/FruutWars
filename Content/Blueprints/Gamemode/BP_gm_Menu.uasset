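; BP_gm_Menu is the game mode for the main menu, setting up its UI and music.
; On BeginPlay it adds the background, main menu and loading screen widgets to the viewport, keeps the loading screen hidden behind a stored reference, and shows the mouse cursor.
; It then has BP_game_Instance start the menu music.
; On EndPlay it removes all widgets.
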(event EventBeginPlay
  (Utilities|FlowControl|Sequence
    (:then_0
      (bind _returnvalue (UserInterface|CreateWidget "/Game/UI/WBP_menu_Background.WBP_menu_Background_C"))
      (UserInterface|Viewport|AddtoViewport _returnvalue 0)
      (bind _returnvalue_2 (UserInterface|CreateWidget "/Game/UI/WBP_menu_MainMenu.WBP_menu_MainMenu_C"))
      (UserInterface|Viewport|AddtoViewport _returnvalue_2 0)
      (bind _returnvalue_3 (UserInterface|CreateWidget "/Game/UI/WBP_game_LoadingScreen.WBP_game_LoadingScreen_C"))
      (bind _output_get (Variables|Default|SetLoadingScreen _returnvalue_3))
      (UserInterface|Viewport|AddtoViewport _output_get 0)
      (Widget|SetVisibility _output_get "Hidden")
      (Variables|/Script/Engine.PlayerController|SetbShowMouseCursor (Game|GetPlayerController 0) true))
    (:then_1
      (bind _asbp_game_instance (Utilities|Casting|CastToBP_game_Instance (Game|GetGameInstance)))
      (Default|PlayMenuMusic _asbp_game_instance))))

(event EventEndPlay
  (params (EndPlayReason :type EEndPlayReason%20Enum :default "Destroyed"))
  (Viewport|RemoveAllWidgets))

(fn ConstructionScript)