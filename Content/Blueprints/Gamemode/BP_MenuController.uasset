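; Menu player controller that handles joining, readying up and Commissioner Potato skin selection, and forwards menu inputs to the menu widget.
; Keyboard or controller join inputs record the device type, call the game mode's JoinGame and assign a free skin.
; Left and right cycle skins with wraparound, skipping any held by other active players, and write materials and portraits to FWPlayerState.
; Character-class cycling is present but unconnected.
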(event Custom|UpdateSkin
  (bind _selectedskin (Variables|Default|GetSelectedSkin))
  ;[1 1 1] updates the ui
  (Variables|/Script/FruutWars.FWPlayerState|SetSelectedSkinHead (Variables|Default|GetFWPlayerState) (Utilities|Array|Get(acopy) (Variables|Default|GetCommPotatoSkinsHead) _selectedskin))
  (Variables|/Script/FruutWars.FWPlayerState|SetSelectedSkinBody (Variables|Default|GetFWPlayerState) (Utilities|Array|Get(acopy) (Variables|Default|GetCommPotatoSkinsBody) _selectedskin))
  (Variables|/Script/FruutWars.FWPlayerState|SetPlayerDisplay (Variables|Default|GetFWPlayerState) (Utilities|Array|Get(acopy) (Variables|Default|GetPlayerDisplays) _selectedskin))
  (Variables|/Script/FruutWars.FWPlayerState|SetPlayerHUDDisplay (Variables|Default|GetFWPlayerState) (Utilities|Array|Get(acopy) (Variables|Default|GetPlayerHUDDisplays) _selectedskin)))

(event EventBeginPlay
  (bind _asbp_gm_menu (Utilities|Casting|CastToBP_gm_Menu (Game|GetGameMode)))
  (Variables|Default|SetGameMode _asbp_gm_menu)
  (Class|CharacterController|DisablePlayerInput)
  (Input|SetInputModeGameandUI self (Variables|/Game/UI/WBP_menu_MainMenu.WBP_menu_MainMenu_C|Getbtn_play (Variables|/Game/Blueprints/Gamemode/BP_gm_Menu.BP_gm_Menu_C|GetMenuBlueprint _asbp_gm_menu)) "DoNotLock" false)
  (Utilities|AddCommPotatoSkins)
  (bind _asfwplayer_state (Utilities|Casting|CastToFWPlayerState (Variables|Default|GetPlayerState)))
  (bind _output_get (Variables|Default|SetFWPlayerState _asfwplayer_state))
  (if (not (Utilities|IsValidClass (Variables|/Script/FruutWars.FWPlayerState|GetSelectedCharacter _output_get)))
    (Variables|/Script/FruutWars.FWPlayerState|SetSelectedCharacter _output_get "/Game/Blueprints/Characters/BP_cha_CommisionerPotato.BP_cha_CommisionerPotato_C")
    (Variables|/Script/FruutWars.FWPlayerState|SetSelectedSkinHead _output_get "/Game/Material/ComPotato/Variant1/MI_ComPotatoAcc_V1.MI_ComPotatoAcc_V1")
    (Variables|/Script/FruutWars.FWPlayerState|SetSelectedSkinBody _output_get "/Game/Material/ComPotato/Variant1/MI_ComPotatoBody_V1.MI_ComPotatoBody_V1")
    (Variables|/Script/FruutWars.FWPlayerState|SetPlayerDisplay _output_get "/Game/UI/Textures/T_menu_CommPotato_1.T_menu_CommPotato_1")
    (Variables|/Script/FruutWars.FWPlayerState|SetPlayerHUDDisplay _output_get "/Game/UI/Textures/T_menu_CommPotatoFace1.T_menu_CommPotatoFace1")))

(event Input|ActionEvents|InputActionMenuUp
  (params (Key :type Key%20Structure))
  (bind _gamemode (Variables|Default|GetGameMode))
  (bind _menublueprint (Variables|/Game/Blueprints/Gamemode/BP_gm_Menu.BP_gm_Menu_C|GetMenuBlueprint _gamemode))
  ;[1 1 1] translate inputs to menu widget
  (:Pressed
    (Utilities|IsValid _menublueprint
      (:Is%20Valid
        (Default|EventMenuUp _menublueprint)))))

(event Input|ActionEvents|InputActionMenuRight
  (params (Key :type Key%20Structure))
  (bind _gamemode (Variables|Default|GetGameMode))
  (bind _menublueprint (Variables|/Game/Blueprints/Gamemode/BP_gm_Menu.BP_gm_Menu_C|GetMenuBlueprint _gamemode))
  ;[1 1 1] translate inputs to menu widget
  (:Pressed
    (Utilities|IsValid _menublueprint
      (:Is%20Valid
        (Default|EventMenuRight _menublueprint)))))

(event Input|ActionEvents|InputActionMenuRight
  (params (Key :type Key%20Structure))
  (bind _commpotatoskinshead (Variables|Default|GetCommPotatoSkinsHead))
  (bind _fwplayerstate (Variables|Default|GetFWPlayerState))
  (bind _returnvalue (Utilities|Array|Length _commpotatoskinshead))
  ;[1 1 1] skin select
  (:Pressed
    (if (Math|Boolean|ANDBoolean (Utilities|Enum|Equal(Enum) (Variables|/Game/Blueprints/Gamemode/BP_gm_Menu.BP_gm_Menu_C|GetMenuState (Variables|Default|GetGameMode)) "NewEnumerator6") (not (Variables|/Script/FruutWars.FWPlayerState|GetIsReady _fwplayerstate)) (!= (Variables|/Script/FruutWars.FWPlayerState|GetGamePlayerIndex _fwplayerstate) -1))
      (Math|Integer|IncrementInt (Variables|Default|GetSelectedSkin) :!label _label
        (:%20%20
          (Variables|Default|SetSelectedSkin (Math|Integer|%(Integer) (+ (Variables|Default|GetSelectedSkin) _returnvalue) _returnvalue))
          (bind _valid (CallFunction|CheckSkinValid))
          (while (not _valid)
            (goto _label))
          (CallFunction|UpdateSkin)
          (Audio|PlaySound2D "/Game/Audio/SFX_MenuTick.SFX_MenuTick" 1.0 1.0 0.0 0 0))))))

(event Input|ActionEvents|InputActionMenuApply
  (params (Key :type Key%20Structure))
  (bind _fwplayerstate (Variables|Default|GetFWPlayerState))
  ;[1 1 1] ready up
  (:Pressed
    (Development|PrintString "applied")
    (if (Variables|/Game/Blueprints/Gamemode/BP_gm_Menu.BP_gm_Menu_C|GetCanPlayerReady (Variables|Default|GetGameMode))
      (if (!= (Variables|/Script/FruutWars.FWPlayerState|GetGamePlayerIndex (Variables|Default|GetFWPlayerState)) -1)
        (Variables|/Script/FruutWars.FWPlayerState|SetIsReady _fwplayerstate (not (Variables|/Script/FruutWars.FWPlayerState|GetIsReady _fwplayerstate)))))))

(event Input|ActionEvents|InputActionMenuLeft
  (params (Key :type Key%20Structure))
  (bind _commpotatoskinshead (Variables|Default|GetCommPotatoSkinsHead))
  (bind _fwplayerstate (Variables|Default|GetFWPlayerState))
  (bind _returnvalue (Utilities|Array|Length _commpotatoskinshead))
  ;[1 1 1] skin select
  (:Pressed
    (if (Math|Boolean|ANDBoolean (Utilities|Enum|Equal(Enum) (Variables|/Game/Blueprints/Gamemode/BP_gm_Menu.BP_gm_Menu_C|GetMenuState (Variables|Default|GetGameMode)) "NewEnumerator6") (not (Variables|/Script/FruutWars.FWPlayerState|GetIsReady _fwplayerstate)) (!= (Variables|/Script/FruutWars.FWPlayerState|GetGamePlayerIndex _fwplayerstate) -1))
      (Math|Integer|DecrementInt (Variables|Default|GetSelectedSkin) :!label _label
        (:%20%20
          (Variables|Default|SetSelectedSkin (Math|Integer|%(Integer) (+ (Variables|Default|GetSelectedSkin) _returnvalue) _returnvalue))
          (bind _valid (CallFunction|CheckSkinValid))
          (while (not _valid)
            (goto _label))
          (CallFunction|UpdateSkin)
          (Audio|PlaySound2D "/Game/Audio/SFX_MenuTick.SFX_MenuTick" 1.0 1.0 0.0 0 0))))))

(event Input|ActionEvents|InputActionMenuUp
  (params (Key :type Key%20Structure))
  ;[1 1 1] skin select
)

(event Input|ActionEvents|InputActionMenuDown
  (params (Key :type Key%20Structure))
  ;[1 1 1] skin select
)

(event Input|ActionEvents|InputActionBecomeActiveKeyboard
  (params (Key :type Key%20Structure))
  ;[1 1 1] join game
  (:Pressed
    (Variables|/Script/FruutWars.FWPlayerState|SetIsUsingKeyboard (Variables|Default|GetFWPlayerState) true)
    (if (== (Variables|/Script/FruutWars.FWPlayerState|GetGamePlayerIndex (Variables|Default|GetFWPlayerState)) -1)
      (bind _asfwbase_game_mode (Utilities|Casting|CastToFWBaseGameMode (Game|GetGameMode)))
      (bind _returnvalue (Class|FWBaseGameMode|JoinGame _asfwbase_game_mode self))
      (if _returnvalue
        (bind _valid (CallFunction|CheckSkinValid :!label _label))
        (while (not _valid)
          (Math|Integer|IncrementInt (Variables|Default|GetSelectedSkin)
            (:%20%20
              (goto _label))))
        (CallFunction|UpdateSkin)))))

(event Input|ActionEvents|InputActionBecomeActiveController
  (params (Key :type Key%20Structure))
  (bind _fwplayerstate (Variables|Default|GetFWPlayerState))
  ;[1 1 1] join game
  (:Pressed
    (Variables|/Script/FruutWars.FWPlayerState|SetIsUsingKeyboard _fwplayerstate false)
    (if (== (Variables|/Script/FruutWars.FWPlayerState|GetGamePlayerIndex _fwplayerstate) -1)
      (bind _asfwbase_game_mode (Utilities|Casting|CastToFWBaseGameMode (Game|GetGameMode)))
      (bind _returnvalue (Class|FWBaseGameMode|JoinGame _asfwbase_game_mode self))
      (if _returnvalue
        (bind _valid (CallFunction|CheckSkinValid :!label _label))
        (while (not _valid)
          (Math|Integer|IncrementInt (Variables|Default|GetSelectedSkin)
            (:%20%20
              (goto _label))))
        (CallFunction|UpdateSkin)))))

(event Input|ActionEvents|InputActionMenuApply
  (params (Key :type Key%20Structure))
  (bind _gamemode (Variables|Default|GetGameMode))
  (bind _menublueprint (Variables|/Game/Blueprints/Gamemode/BP_gm_Menu.BP_gm_Menu_C|GetMenuBlueprint _gamemode))
  ;[1 1 1] translate inputs to menu widget
  (:Pressed
    (Utilities|IsValid _menublueprint
      (:Is%20Valid
        (Default|EventMenuApply _menublueprint)))))

(event Input|ActionEvents|InputActionMenuBack
  (params (Key :type Key%20Structure))
  (bind _gamemode (Variables|Default|GetGameMode))
  (bind _menublueprint (Variables|/Game/Blueprints/Gamemode/BP_gm_Menu.BP_gm_Menu_C|GetMenuBlueprint _gamemode))
  ;[1 1 1] translate inputs to menu widget
  (:Pressed
    (Utilities|IsValid _menublueprint
      (:Is%20Valid
        (Default|EvenMenuBack _menublueprint)))))

(event Input|ActionEvents|InputActionMenuDown
  (params (Key :type Key%20Structure))
  (bind _gamemode (Variables|Default|GetGameMode))
  (bind _menublueprint (Variables|/Game/Blueprints/Gamemode/BP_gm_Menu.BP_gm_Menu_C|GetMenuBlueprint _gamemode))
  ;[1 1 1] translate inputs to menu widget
  (:Pressed
    (Utilities|IsValid _menublueprint
      (:Is%20Valid
        (Default|EventMenuDown _menublueprint)))))

(event Input|ActionEvents|InputActionMenuLeft
  (params (Key :type Key%20Structure))
  (bind _gamemode (Variables|Default|GetGameMode))
  (bind _menublueprint (Variables|/Game/Blueprints/Gamemode/BP_gm_Menu.BP_gm_Menu_C|GetMenuBlueprint _gamemode))
  ;[1 1 1] translate inputs to menu widget
  (:Pressed
    (Utilities|IsValid _menublueprint
      (:Is%20Valid
        (Default|EventMenuLeft _menublueprint)))))

(fn ConstructionScript)

(fn CheckSkinValid
  (for _array_element (Variables|/Script/FruutWars.FWBaseGameMode|GetActivePlayers (Variables|Default|GetGameMode))
    (if (and (!= _array_element self) (Utilities|IsValid _array_element))
      (bind _asbp_menu_controller (Utilities|Casting|CastToBP_MenuController _array_element))
      (if (== (Variables|BP_MenuController_C|GetSelectedSkin _asbp_menu_controller) (Variables|Default|GetSelectedSkin))
        (return false))))
  (return true))