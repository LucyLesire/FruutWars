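; Game instance for FruutWars that owns the background music for menus and gameplay, keeping it alive across level transitions.
; On Init it creates persistent 2D audio components for two menu tracks and one gameplay track.
; Finished-audio events alternate the menu tracks and loop the gameplay track.
; Play events switch between menu and game music without restarting music already playing, and StopMusic stops all tracks.
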(event Custom|PlayMenuMusic
  (Audio|Components|Audio|Stop (Variables|Default|GetGameMusic))
  (if (and (not (Audio|Components|Audio|IsPlaying (Variables|Default|GetMenuMusic1))) (not (Audio|Components|Audio|IsPlaying (Variables|Default|GetMenuMusic2))))
    (Audio|Components|Audio|Play (Variables|Default|GetMenuMusic2) 0.0)))

(event Custom|Menu1End
  (Audio|Components|Audio|Play (Variables|Default|GetMenuMusic2) 0.0))

(event Custom|Menu2End
  (Audio|Components|Audio|Play (Variables|Default|GetMenuMusic1) 0.0))

(event Custom|GameMusicEnd
  (Audio|Components|Audio|Play (Variables|Default|GetGameMusic) 0.0))

(event Custom|PlayGameMusic
  (Audio|Components|Audio|Stop (Variables|Default|GetMenuMusic2))
  (Audio|Components|Audio|Stop (Variables|Default|GetMenuMusic1))
  (if (not (Audio|Components|Audio|IsPlaying (Variables|Default|GetGameMusic)))
    (Audio|Components|Audio|Play (Variables|Default|GetGameMusic) 0.0)))

(event Custom|StopMusic
  (Audio|Components|Audio|Stop (Variables|Default|GetMenuMusic2))
  (Audio|Components|Audio|Stop (Variables|Default|GetMenuMusic1))
  (Audio|Components|Audio|Stop (Variables|Default|GetGameMusic)))

(event EventInit
  (bind _returnvalue (Audio|CreateSound2D "/Game/Audio/Music/Main_Menu/FruutWars_MainMenuMusic_01.FruutWars_MainMenuMusic_01" 1.0 1.0 0.0 0 true false))
  (Variables|Default|SetMenuMusic1 _returnvalue)
  (bind _returnvalue_2 (Audio|CreateSound2D "/Game/Audio/Music/Main_Menu/FruutWars_MainMenuMusic_02.FruutWars_MainMenuMusic_02" 1.0 1.0 0.0 0 true false))
  (Variables|Default|SetMenuMusic2 _returnvalue_2)
  (bind _returnvalue_3 (Audio|CreateSound2D "/Game/Audio/Music/GamePlay/FruutWars_GameplayLoopMusic_01.FruutWars_GameplayLoopMusic_01" 1.0 1.0 0.0 0 true false))
  (Variables|Default|SetGameMusic _returnvalue_3)
  (EventDispatchers|BindEventtoOnAudioFinished (Variables|Default|GetMenuMusic1) (delegate Custom|Menu1End))
  (EventDispatchers|BindEventtoOnAudioFinished (Variables|Default|GetMenuMusic2) (delegate Custom|Menu2End))
  (EventDispatchers|BindEventtoOnAudioFinished (Variables|Default|GetGameMusic) (delegate Custom|GameMusicEnd)))