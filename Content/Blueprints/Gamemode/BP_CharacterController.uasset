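; Player controller for the free-for-all mode that enables player input on begin play and handles pausing.
; The PauseGame input casts the game mode to BP_gm_FreeForAll and calls PauseGame on its PauseScreen.
; The construction script sets PlayerClass to the Commisioner Potato character.
; Disconnected, never-run nodes hold older or unused logic for spawning and possessing Potato or Jalapeno characters and creating the HUD widget.
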(event EventBeginPlay
  (Class|CharacterController|EnablePlayerInput))

(event Input|ActionEvents|InputActionPauseGame
  (params (Key :type Key%20Structure :default "None"))
  (:Pressed
    (bind _asbp_gm_free_for_all (Utilities|Casting|CastToBP_gm_FreeForAll (Game|GetGameMode)))
    (Default|PauseGame (Variables|/Game/Blueprints/Gamemode/BP_gm_FreeForAll.BP_gm_FreeForAll_C|GetPauseScreen _asbp_gm_free_for_all))))

(event Input|GamepadEvents|GamepadSpecialLeft
  (params (Key :type Key%20Structure :default "None")))

(event Input|KeyboardEvents|I
  (params (Key :type Key%20Structure :default "None")))

(fn ConstructionScript
  (Variables|Default|SetPlayerClass "/Game/Blueprints/Characters/BP_cha_CommisionerPotato.BP_cha_CommisionerPotato_C"))