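; Free-for-all game mode that runs rounds on sinking tiles until a player reaches the winning score.
; BeginPlay registers weighted tiles, creates UI widgets, spawns skinned players and locks input until the countdown ends and sinking starts.
; RestartRound shows results, then seamlessly travels to reload the level, or to the main menu after a win.
; Events toggle tile shaking and briefly slow time on player death.
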(event Custom|countdownEnd
  (Class|FWBaseGameMode|EnableAllPlayerInput)
  (Class|FWBaseGameMode|GetTile)
  (Variables|Default|SetbSinkTiles true))

(event EventBeginPlay
  (bind _spawnlocations (Variables|Default|GetSpawnLocations))
  (|CallParentFunction)
  (Utilities|FlowControl|Sequence
    (:then_0
      (Viewport|RemoveAllWidgets)
      (Class|FWBaseGameMode|InitializeTiles)
      (Utilities|InitializeWidgets)
      (Utilities|FlowControl|Delay 0.2)
      ;[1 1 1] spawn players
      (bind _outactors (Actor|GetAllActorsOfClass "/Script/FruutWars.SpawnPoint"))
      (bind _output_get (Variables|Default|SetoutSpawnPoints _outactors))
      (for _array_element _output_get
        (Utilities|Array|Add _spawnlocations (Transformation|GetActorLocation _array_element)))
      (Class|FWBaseGameMode|SpawnPlayers _spawnlocations)
      (for _array_element_2 (Variables|Default|GetActivePlayers)
        (Utilities|IsValid _array_element_2
          (:Is%20Valid
            (bind _ascharacter (Utilities|Casting|CastToCharacter (Pawn|GetControlledPawn _array_element_2)))
            (bind _asfwplayer_state (Utilities|Casting|CastToFWPlayerState (Variables|/Script/Engine.Pawn|GetPlayerState _ascharacter)))
            (Rendering|Material|SetMaterial (Variables|/Script/Engine.Character|GetMesh _ascharacter) 0 (Variables|/Script/FruutWars.FWPlayerState|GetSelectedSkinHead _asfwplayer_state))
            (Rendering|Material|SetMaterial (Variables|/Script/Engine.Character|GetMesh _ascharacter) 1 (Variables|/Script/FruutWars.FWPlayerState|GetSelectedSkinBody _asfwplayer_state))
            (Rendering|SetCustomDepthStencilValue (Variables|/Script/Engine.Character|GetMesh _ascharacter) (+ (Variables|/Script/FruutWars.FWPlayerState|GetGamePlayerIndex _asfwplayer_state) 1))
            (bind _asbp_cha_base_char (Utilities|Casting|CastToBP_cha_BaseChar _ascharacter))
            (Variables|/Game/Blueprints/Characters/BP_cha_BaseChar.BP_cha_BaseChar_C|SetplayerController _asbp_cha_base_char _array_element_2))))
      (Class|FWBaseGameMode|DisableAllPlayerInput)
      (Default|StartCountdown (Variables|Default|GetCountdown))
      ;[1 1 1] Initialize HUD
      (bind _asbp_hud (Utilities|Casting|CastToBP_HUDClass (Variables|Default|GetHUDClass)))
      (bind _returnvalue (Actor|GetActorOfClass _asbp_hud))
      (EventDispatchers|BindEventtoOnCountdownEnd (Variables|Default|GetCountdown) (delegate Custom|countdownEnd)))
    (:then_1
      (bind _asbp_game_instance (Utilities|Casting|CastToBP_game_Instance (Game|GetGameInstance)))
      (Default|PlayGameMusic _asbp_game_instance))))

(event EventTick
  (params (DeltaSeconds :type Float%20%28single-precision%29))
  (|CallParentFunction 0.0))

(event EventInitializeTiles
  ;[1 1 1] Init Tiles
  (bind _outactors (Actor|GetAllActorsOfClasswithTag "/Game/Blueprints/LevelMechanics/BP_env_Tile.BP_env_Tile_C" "Movable"))
  (for _array_element _outactors
    (Utilities|Map|Add (Variables|Default|GetTileWeights) _array_element (Variables|/Game/Blueprints/LevelMechanics/BP_env_Tile.BP_env_Tile_C|GetWeight _array_element))))

(event EventRestartRound
  (bind _endofroundscreen (Variables|Default|GetEndOfRoundScreen))
  (Class|FWBaseGameMode|DisableAllPlayerInput)
  (Utilities|FlowControl|Delay 1.5)
  (Widget|SetVisibility _endofroundscreen "Visible")
  (Default|UpdateInfo _endofroundscreen)
  (Utilities|FlowControl|Delay 4.0)
  (for _array_element (Variables|Default|GetActivePlayers)
    (Utilities|IsValid _array_element
      (:Is%20Valid
        (bind _asfwplayer_state (Utilities|Casting|CastToFWPlayerState (Variables|/Script/Engine.Controller|GetPlayerState _array_element)))
        (if (>= (Variables|/Script/FruutWars.FWPlayerState|GetFWRoundScore _asfwplayer_state) (Variables|Default|GetWinningScore))
          (Variables|Default|SetHasPlayerWon true)
          (Default|SetWonPlayer (Variables|Default|GetPlayerWin) _asfwplayer_state)))))
  (Widget|SetVisibility (Variables|Default|GetEndOfRoundScreen) "Hidden")
  (if (Variables|Default|GetHasPlayerWon)
    (Widget|SetVisibility (Variables|Default|GetPlayerWin) "Visible")
    (Utilities|FlowControl|Delay 5.0)
    (Widget|SetVisibility (Variables|Default|GetLoadingScreen) "Visible")
    (Widget|SetVisibility (Variables|Default|GetPlayerWin) "Hidden")
    (Class|FWBaseGameMode|SeamlessTravel "LVL_menu_MainMenu")
    (else
      (bind _returnvalue (Game|GetCurrentLevelName true))
      (Widget|SetVisibility (Variables|Default|GetLoadingScreen) "Visible")
      (Class|FWBaseGameMode|SeamlessTravel _returnvalue))))

(event EventOnPlayerDied
  ;[1 1 1] time dilation
  (Utilities|Time|SetGlobalTimeDilation 0.2)
  (Utilities|FlowControl|Delay 0.2)
  (Utilities|Time|SetGlobalTimeDilation 1.0))

(event EventStartTileShake
  (params (tile :type Actor%20Object%20Reference))
  (bind _asbp_env_tile (Utilities|Casting|CastToBP_env_Tile tile))
  (Variables|/Game/Blueprints/LevelMechanics/BP_env_Tile.BP_env_Tile_C|SetisShaking _asbp_env_tile true))

(event EventStopTileShake
  (params (tile :type Actor%20Object%20Reference))
  (bind _asbp_env_tile (Utilities|Casting|CastToBP_env_Tile tile))
  (Variables|/Game/Blueprints/LevelMechanics/BP_env_Tile.BP_env_Tile_C|SetisShaking _asbp_env_tile false))

(fn ConstructionScript)