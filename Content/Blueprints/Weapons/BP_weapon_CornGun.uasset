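; Corn gun weapon Blueprint that adds its own muzzle effect and firing sound to inherited weapon behavior.
; On BeginPlay it binds to the OnShoot dispatcher, which spawns the Niagara muzzle flash at the Shootmuzzle component's transform.
; Its OnWeaponFire override calls the parent logic, then plays the corn shotgun sound at the weapon's root location.
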(event Custom|SpawnMuzzle
  (bind _shootmuzzle (Variables|Default|Getshootmuzzle))
  (Niagara|SpawnSystematLocation "/Game/RFX/Emitters/FXS_Cornun_Muzzle.FXS_Cornun_Muzzle" (Transformation|GetWorldLocation _shootmuzzle) (Transformation|GetSocketRotation _shootmuzzle "None") (Transformation|GetWorldScale _shootmuzzle)))

(event EventBeginPlay
  (EventDispatchers|BindEventtoOnShoot (delegate Custom|SpawnMuzzle)))

(event Collision|EventActorBeginOverlap
  (params (OtherActor :type Actor%20Object%20Reference)))

(event EventTick
  (params (DeltaSeconds :type Float%20%28single-precision%29)))

(event EventOnWeaponFire
  (params (direction :type Vector%20%28by%20ref%29 :default "0, 0, 0"))
  (|CallParentFunction direction)
  (Audio|SpawnSoundatLocation "/Game/Audio/SFX_CornShotGunShoot.SFX_CornShotGunShoot" (Transformation|GetWorldLocation (Variables|Transformation|GetRootComponent)) "0, 0, 0" 1.0 1.0 0.0 0 0))

(fn ConstructionScript)