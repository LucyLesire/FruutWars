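; BP_env_camera is a shared environment camera that frames all active players from one view.
; Until found, it polls player controllers on Tick and sets itself as their view target.
; It then moves to the players' center from FWBaseGameMode, snapping back to its start location when that center is nearly there or too far away.
; The follow camera's arm length eases toward a clamped multiple of the furthest player distance, zooming with player spread.
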(event EventBeginPlay
  (bind _asfwbase_game_mode (Utilities|Casting|CastToFWBaseGameMode (Game|GetGameMode)))
  (Variables|Default|SetGameMode _asfwbase_game_mode)
  (Variables|Default|SetOriginalLocation (Transformation|GetActorLocation)))

(event EventTick
  (params (DeltaSeconds :type Float%20%28single-precision%29))
  (if (Variables|Default|GetFoundPlayer)
    (for _array_element (Variables|/Script/FruutWars.FWBaseGameMode|GetActivePlayers (Variables|Default|GetGameMode))
      (bind _returnvalue (Class|FWBaseGameMode|GetCenterOfPlayers (Variables|Default|GetGameMode)))
      (if (or (< (Math|Vector|Distance(Vector) _returnvalue (Variables|Default|GetOriginalLocation)) 1.0) (> (Math|Vector|Distance(Vector) _returnvalue (Variables|Default|GetOriginalLocation)) 5e+03))
        (Transformation|SetActorLocation (Variables|Default|GetOriginalLocation) false false)
        (else
          (Transformation|SetActorLocation _returnvalue false false)))
      (bind _returnvalue_2 (Class|FWBaseGameMode|GetFurthestDistancefromPlayers (Variables|Default|GetGameMode) _returnvalue))
      (Variables|/Script/Engine.SpringArmComponent|SetTargetArmLength (Variables|Default|GetFollowCamera) (Math|Float|Clamp(Float) (Math|Interpolation|FInterpTo (Variables|/Script/Engine.SpringArmComponent|GetTargetArmLength (Variables|Default|GetFollowCamera)) (* _returnvalue_2 4.0) (Utilities|Time|GetWorldDeltaSeconds) 1.0) 2.5e+03 4e+03)))
    (else
      (bind _returnvalue_3 (Class|GameModeBase|GetNumPlayers (Game|GetGameMode)))
      (for _index (range 0 _returnvalue_3)
        (Utilities|IsValid (Game|GetPlayerController _index)
          (:Is%20Valid
            (Game|Player|SetViewTargetwithBlend (Game|GetPlayerController _index) self 0.0 "VTBlend_Linear" 0.0 false)
            (Variables|Default|SetFoundPlayer true)))))))

(fn ConstructionScript)