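; BP_env_Water is a water hazard that kills characters falling into it.
; On actor overlap, a BaseCharacter is killed through its HealthComponent, with a splash sound and Niagara effect spawned at its transform.
; BP_proj_CocunutBall projectiles are destroyed on overlap or on hitting the Box component.
; A delayed cleanup of the splash effect is present but unconnected, so it never runs.
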(event OnComponentHit(Box)
  (params (HitComponent :type Primitive%20Component%20Object%20Reference) (OtherActor :type Actor%20Object%20Reference) (OtherComp :type Primitive%20Component%20Object%20Reference) (NormalImpulse :type Vector :default "0, 0, 0") (Hit :type Hit%20Result%20Structure%20%28by%20ref%29))
  (bind _asbp_proj_cocunut_ball (Utilities|Casting|CastToBP_proj_CocunutBall OtherActor))
  (Actor|DestroyActor _asbp_proj_cocunut_ball))

(event Collision|EventActorBeginOverlap
  (params (OtherActor :type Actor%20Object%20Reference))
  (Utilities|IsValid OtherActor
    (:Is%20Valid
      (bind _asbase_character (Utilities|Casting|CastToBaseCharacter OtherActor)
        (:then
          (Class|HealthComponent|DoKill (Variables|/Script/FruutWars.BaseCharacter|GetHealthComponent _asbase_character))
          (Audio|SpawnSoundatLocation "/Game/Audio/WaterSplash.WaterSplash" (.location (Transformation|GetActorTransform _asbase_character)) "0, 0, 0" 1.0 1.0 0.0 0 0)
          (bind _returnvalue (Niagara|SpawnSystematLocation "/Game/RFX/System/FXS_env_watersplash.FXS_env_watersplash" (.location (Transformation|GetActorTransform _asbase_character)) (.rotation (Transformation|GetActorTransform _asbase_character)) (.scale (Transformation|GetActorTransform _asbase_character)))))
        (:CastFailed
          (bind _asbp_proj_cocunut_ball (Utilities|Casting|CastToBP_proj_CocunutBall (stale OnComponentHit(Box) OtherActor)))
          (Actor|DestroyActor _asbp_proj_cocunut_ball))))))

(event EventTick
  (params (DeltaSeconds :type Float%20%28single-precision%29)))

(fn ConstructionScript)