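; BP_env_FloatingText is a short-lived actor that displays coloured floating text in the level through a WBP_FloatingText widget.
; On BeginPlay it moves up by a fixed amount plus a small random offset.
; Initialize sets the screen time and passes the text and colour to the widget.
; Tick counts the remaining time down and destroys the actor when it runs out.
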(event Custom|Initialize
  (params (time%20on%20screen :type Float%20%28single-precision%29) (text :type Text) (color :type Linear%20Color%20Structure))
  (Variables|Default|SetTimeRemaining time%20on%20screen)
  (bind _aswbp_floating_text (Utilities|Casting|CastToWBP_FloatingText (UserInterface|GetWidget (Variables|Default|GetText))))
  (Variables|/Game/UI/WBP_FloatingText.WBP_FloatingText_C|SetText _aswbp_floating_text text)
  (Variables|/Game/UI/WBP_FloatingText.WBP_FloatingText_C|SetColor _aswbp_floating_text color))

(event EventBeginPlay
  (Transformation|AddActorLocalOffset (+ (* (Math|Random|RandomUnitVector) 25.0) "0.000000,0.000000,40.000000") false false))

(event EventTick
  (params (DeltaSeconds :type Float%20%28single-precision%29))
  (bind _output_get (Variables|Default|SetTimeRemaining (- (Variables|Default|GetTimeRemaining) DeltaSeconds)))
  (if (<= _output_get 0.0)
    (Actor|DestroyActor)))

(fn ConstructionScript)