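; BP_env_Tile is a level tile that rumbles when shaking and splashes on contact with water.
; When IsShaking, set outside these graphs, first turns on, Tick plays a sound and world camera shake once, as WasShaking is never reset here.
; While shaking, Tick starts looping force feedback for overlapping characters, stopped when they leave.
; Box ending overlap with BP_env_Water spawns a splash effect and randomly pitched sound.
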(event OnComponentEndOverlap(Box)
  (params (OverlappedComponent :type Primitive%20Component%20Object%20Reference) (OtherActor :type Actor%20Object%20Reference) (OtherComp :type Primitive%20Component%20Object%20Reference) (OtherBodyIndex :type Integer))
  (bind _returnvalue (Transformation|GetActorTransform))
  (Utilities|IsValid OtherActor
    (:Is%20Valid
      (Utilities|Casting|CastToBP_env_Water OtherActor)
      (Niagara|SpawnSystematLocation "/Game/RFX/System/FXS_env_watersplash.FXS_env_watersplash" (.location _returnvalue) (.rotation _returnvalue) (Variables|Default|GetSplashScale))
      (Audio|PlaySoundatLocation "/Game/Audio/WaterSplash.WaterSplash" (Transformation|GetWorldLocation (Variables|Default|GetBox)) "0, 0, 0" 1.0 (Math|Random|RandomFloatinRange 0.01 0.4) 0.4 0 0 0))))

(event EventBeginPlay)

(event EventTick
  (params (DeltaSeconds :type Float%20%28single-precision%29))
  (bind _returnvalue (Transformation|GetActorLocation))
  ;[1 1 1] Play rumble effect
  (if (and (not (Variables|Default|GetwasShaking)) (Variables|Default|GetisShaking))
    (Audio|PlaySoundatLocation (Variables|Default|GetRumbleSound) _returnvalue "0, 0, 0" 1.0 1.0 0.0 0 0 0)
    (Variables|Default|SetwasShaking true)
    (Camera|PlayWorldCameraShake "/Game/Blueprints/LevelMechanics/BP_TileShake.BP_TileShake_C" _returnvalue 0.0 1e+04 3.0))
  (if (Variables|Default|GetisShaking)
    (Utilities|FlowControl|Sequence
      (:then_0
        (for _array_element (Variables|Default|GetoverlappingPlayers)
          (Game|Feedback|ClientPlayForceFeedback (Variables|/Game/Blueprints/Characters/BP_cha_BaseChar.BP_cha_BaseChar_C|GetplayerController _array_element) "/Game/Audio/TileRumble.TileRumble" "TileRumble" true false false))))))

(event Collision|EventActorBeginOverlap
  (params (OtherActor :type Actor%20Object%20Reference))
  ;[1 1 1] Add Player to rumble effect
  (bind _asbp_cha_base_char (Utilities|Casting|CastToBP_cha_BaseChar OtherActor))
  (Utilities|Array|AddUnique (Variables|Default|GetoverlappingPlayers) _asbp_cha_base_char))

(event Collision|EventActorEndOverlap
  (params (OtherActor :type Actor%20Object%20Reference))
  ;[1 1 1] Add Player to rumble effect
  (bind _asbp_cha_base_char (Utilities|Casting|CastToBP_cha_BaseChar OtherActor))
  (Utilities|Array|RemoveItem (Variables|Default|GetoverlappingPlayers) _asbp_cha_base_char)
  (Game|Feedback|ClientStopForceFeedback (Variables|/Game/Blueprints/Characters/BP_cha_BaseChar.BP_cha_BaseChar_C|GetplayerController _asbp_cha_base_char) "/Game/Audio/TileRumble.TileRumble" "TileRumble"))

(fn ConstructionScript)