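; Test destructible crate that shows floating damage numbers and breaks apart on death.
; BeginPlay binds the HealthComponent's damage event to spawn floating text, colored blue while shield remains and white otherwise.
; OnDeath hides the mesh, disables its collision, spawns a plank Niagara effect and, if MakeSound is set, plays a break sound with randomized volume and pitch.
; The swap to a destroyed-crate mesh is left unwired.
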(event Custom|Show%20Text
  (params (DamageAmount :type Float%20%28single-precision%29) (Source :type Controller%20Object%20Reference))
  (bind _returnvalue (Utilities|Text|ToText(Float) DamageAmount "HalfToEven" false true 1 324 0 0))
  (bind _returnvalue_2 (Game|SpawnActorfromClass "/Game/Blueprints/LevelMechanics/BP_env_FloatingText.BP_env_FloatingText_C" (Math|Conversions|ToTransform(Vector) (Transformation|GetActorLocation)) "Undefined" 0 0))
  (if (> (Variables|/Script/FruutWars.HealthComponent|GetCurrentShield (Variables|Default|GetHealthComponent)) 0.0)
    (Default|Initialize _returnvalue_2 0.5 _returnvalue "(R=0.000000,G=0.509804,B=1.000000,A=1.000000)")
    (else
      (Default|Initialize _returnvalue_2 0.5 _returnvalue "(R=1.000000,G=1.000000,B=1.000000,A=1.000000)"))))

(event EventBeginPlay
  (EventDispatchers|BindEventtoOnDamage (Variables|Default|GetHealthComponent) (delegate Custom|Show%20Text)))

(event EventOnDeath
  (bind _returnvalue (Transformation|GetActorLocation))
  (bind _returnvalue_2 (Math|Random|RandomFloatinRange 0.9 1.1))
  (Rendering|SetVisibility (Variables|Default|GetStaticMesh) false false)
  (Collision|SetCollisionEnabled (Variables|Default|GetStaticMesh) "NoCollision")
  (Niagara|SpawnSystematLocation "/Game/RFX/System/FXE_Planks2_System.FXE_Planks2_System" (Transformation|GetActorLocation) "0, 0, 0" "1.000000,1.000000,1.000000" true true "AutoRelease")
  (if (Variables|Default|GetmakeSound)
    (switch int (Math|Random|RandomInteger 4)
      (:0
        (Audio|PlaySoundatLocation "/Game/Audio/500902__bertsz__wood-crate-destory-1.500902__bertsz__wood-crate-destory-1" _returnvalue "0, 0, 0" _returnvalue_2 _returnvalue_2 0.0 0 0 0))
      (:1
        (Audio|PlaySoundatLocation "/Game/Audio/500902__bertsz__wood-crate-destory-1.500902__bertsz__wood-crate-destory-1" _returnvalue "0, 0, 0" _returnvalue_2 _returnvalue_2 0.0 0 0 0))
      (:2
        (Audio|PlaySoundatLocation "/Game/Audio/500902__bertsz__wood-crate-destory-1.500902__bertsz__wood-crate-destory-1" _returnvalue "0, 0, 0" _returnvalue_2 _returnvalue_2 0.0 0 0 0))
      (:3
        (Audio|PlaySoundatLocation "/Game/Audio/SFX_Krate_burst.SFX_Krate_burst" _returnvalue "0, 0, 0" _returnvalue_2 _returnvalue_2 0.0 0 0 0)))))

(fn ConstructionScript)