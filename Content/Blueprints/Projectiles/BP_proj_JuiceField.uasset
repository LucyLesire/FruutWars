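; Lemon juice field that drops to the ground and damages characters standing in it until it expires.
; Shortly after BeginPlay, a downward trace moves the Cylinder to the surface, a pool sound plays, and the actor destroys itself after LifeDuration.
; Cylinder overlaps deal damage on entry and maintain parallel arrays of characters and timers.
; Tick advances each timer, reapplying damage and resetting it whenever MaxTimeBetweenDamage is exceeded.
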(event OnComponentBeginOverlap(Cylinder)
  (params (OverlappedComponent :type Primitive%20Component%20Object%20Reference) (OtherActor :type Actor%20Object%20Reference) (OtherComp :type Primitive%20Component%20Object%20Reference) (OtherBodyIndex :type Integer) (bFromSweep :type Boolean) (SweepResult :type Hit%20Result%20Structure%20%28by%20ref%29))
  ;[1 1 1] Check if player(s) are on the juice field
  (Utilities|IsValid OtherActor
    (:Is%20Valid
      (bind _asbase_character (Utilities|Casting|CastToBaseCharacter OtherActor))
      (Utilities|Array|Add (Variables|Characters|GetCharacters) _asbase_character)
      (Utilities|Array|Add (Variables|Damage|GetTimeBetweenDamage) 0.0)
      (Class|HealthComponent|DoDamage (Variables|/Script/FruutWars.BaseCharacter|GetHealthComponent _asbase_character) (Variables|Damage|GetJuiceFieldDamageAmount) 0))))

(event OnComponentEndOverlap(Cylinder)
  (params (OverlappedComponent :type Primitive%20Component%20Object%20Reference) (OtherActor :type Actor%20Object%20Reference) (OtherComp :type Primitive%20Component%20Object%20Reference) (OtherBodyIndex :type Integer))
  ;[1 1 1] Check if player(s) are on the juice field
  (Utilities|IsValid OtherActor
    (:Is%20Valid
      (bind _asbase_character (Utilities|Casting|CastToBaseCharacter OtherActor))
      (if (!= (Utilities|Array|FindItem (Variables|Characters|GetCharacters) _asbase_character) -1)
        (Utilities|Array|RemoveIndex (Variables|Damage|GetTimeBetweenDamage) (Utilities|Array|FindItem (Variables|Characters|GetCharacters) _asbase_character))
        (Utilities|Array|RemoveIndex (Variables|Characters|GetCharacters) (Utilities|Array|FindItem (Variables|Characters|GetCharacters) _asbase_character))))))

(event EventBeginPlay
  (bind _cylinder (Variables|Default|GetCylinder))
  (bind _returnvalue (Transformation|GetWorldLocation _cylinder))
  ;[1 1 1] Drop Juicefield
  (Utilities|FlowControl|Delay 0.01)
  (bind _outhit (Collision|LineTraceByChannel (Math|Vector|MakeVector (.x _returnvalue) (.y _returnvalue) (.z _returnvalue)) (Math|Vector|MakeVector (.x _returnvalue) (.y _returnvalue) (- (.z _returnvalue) 8e+02)) "TraceTypeQuery1" false 0 "None"))
  (Transformation|SetWorldLocation (Variables|Default|GetCylinder) (.Location (Collision|BreakHitResult _outhit)) false false)
  (Audio|SpawnSoundatLocation "/Game/Audio/SFX_Lemon_Pool.SFX_Lemon_Pool" (Transformation|GetActorLocation) "0, 0, 0" 1.0 1.0 0.0 0 0)
  (Utilities|FlowControl|Delay (Variables|LifeTime|GetLifeDuration))
  (Actor|DestroyActor))

(event EventTick
  (params (DeltaSeconds :type Float%20%28single-precision%29))
  ;[1 1 1] Damage over time
  (for (_array_element _array_index) (Variables|Characters|GetCharacters)
    (Utilities|Array|SetArrayElem (Variables|Damage|GetTimeBetweenDamage) _array_index (+ (Utilities|Array|Get(acopy) (Variables|Damage|GetTimeBetweenDamage) _array_index) DeltaSeconds))
    (if (> (+ (Utilities|Array|Get(acopy) (Variables|Damage|GetTimeBetweenDamage) _array_index) DeltaSeconds) (Variables|Damage|GetMaxTimeBetweenDamage))
      (Class|HealthComponent|DoDamage (Variables|/Script/FruutWars.BaseCharacter|GetHealthComponent _array_element) (Variables|Damage|GetJuiceFieldDamageAmount) 0)
      (Utilities|Array|SetArrayElem (Variables|Damage|GetTimeBetweenDamage) _array_index 0.0))))

(fn ConstructionScript)