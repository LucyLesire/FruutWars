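; Coconut ball projectile that tumbles at a random spin and stuns characters it hits, including the thrower's team after a half-second grace period.
; Character hits trigger the stun effect, spawn impact VFX and sound, then destroy the ball.
; Bounces play a sound, a brief rumble timeline and a delayed world camera shake.
; Tick updates distance-scaled force feedback, but the per-player loop that starts it is unwired.
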(event Custom|on%20bounce
  (params (ImpactResult :type Hit%20Result%20Structure%20%28by%20ref%29) (ImpactVelocity :type Vector%20%28by%20ref%29))
  (bind _projectilerumble (Variables|Default|GetProjectileRumble))
  (Audio|Components|Audio|Play _projectilerumble 0.0)
  (Audio|SpawnSoundatLocation "/Game/Audio/SFX_Coconut_Bounce.SFX_Coconut_Bounce" (Transformation|GetActorLocation) "0, 0, 0" 1.0 1.0 0.0 0 0)
  (Utilities|FlowControl|Delay 0.1)
  (Camera|PlayWorldCameraShake "/Game/Blueprints/Projectiles/BP_CoconutShake.BP_CoconutShake_C" (Transformation|GetActorLocation) 0.0 6e+03)
  (Audio|Components|Audio|Stop _projectilerumble))

(event EventTick
  (params (DeltaSeconds :type Float%20%28single-precision%29))
  (Game|Feedback|PlayDynamicForceFeedback (stale _array_element) (Math|Float|Clamp(Float) (/ (- 2.5e+02 (Math|Vector|Distance(Vector) (Transformation|GetActorLocation (Pawn|GetControlledPawn (stale _array_element))) (Transformation|GetActorLocation self))) 2.5e+02)) 0.1 true true true true) ; enters at Update
)

(event EventOnProjectileHitTeam
  (params (target :type Base%20Character%20Object%20Reference))
  (bind _returnvalue (Transformation|GetActorLocation))
  (bind _stunduration (Variables|Default|GetStunDuration))
  ;[1 1 1] Stun self (Small delay so u don't hit yourself instantly when throwing)
  (if (not (<= (Variables|Default|GetTimeAlive) 0.5))
    (Utilities|IsValid target
      (:Is%20Valid
        (bind _asbp_character_controller (Utilities|Casting|CastToBP_CharacterController (Pawn|GetController target)))
        (Class|CharacterController|Stun _asbp_character_controller _stunduration)
        (bind _asbp_cha_base_char (Utilities|Casting|CastToBP_cha_BaseChar target))
        (Default|ActivateStunEffect _asbp_cha_base_char _stunduration)
        (Audio|Components|Audio|Stop (Variables|Default|GetProjectileRumble))
        (Niagara|SpawnSystematLocation "/Game/RFX/System/FXS_BiggerImpact.FXS_BiggerImpact" _returnvalue)
        (Audio|SpawnSoundatLocation "/Game/Audio/SFX_CoconutBonk.SFX_CoconutBonk" _returnvalue "0, 0, 0" 1.0 1.0 0.5 0 0)
        (Actor|DestroyActor)))))

(event EventDestroyed
  (Niagara|SpawnSystematLocation "/Game/RFX/System/FXS_BiggerImpact.FXS_BiggerImpact" (Transformation|GetActorLocation))
  (Audio|Components|Audio|Stop (Variables|Default|GetProjectileRumble)))

(event EventBeginPlay
  (bind _returnvalue (Math|Random|RandomFloatinRange -1e+02 1e+02))
  (Variables|/Script/Engine.RotatingMovementComponent|SetRotationRate (Variables|Default|GetRotatingMovement) (Math|Rotator|MakeRotator _returnvalue (Math|Random|RandomFloatinRange -3.5e+02 -2.5e+02) _returnvalue))
  (EventDispatchers|BindEventtoOnProjectileBounce (Variables|Default|GetProjectileComponent) (delegate Custom|on%20bounce)))

(event EventOnProjectileHitCharacter
  (params (target :type Base%20Character%20Object%20Reference))
  (bind _returnvalue (Transformation|GetActorLocation))
  (bind _stunduration (Variables|Default|GetStunDuration))
  ;[1 1 1] Stun other player
  (Utilities|IsValid target
    (:Is%20Valid
      (bind _asbp_character_controller (Utilities|Casting|CastToBP_CharacterController (Pawn|GetController target)))
      (Class|CharacterController|Stun _asbp_character_controller _stunduration)
      (bind _asbp_cha_base_char (Utilities|Casting|CastToBP_cha_BaseChar target))
      (Default|ActivateStunEffect _asbp_cha_base_char _stunduration)
      (Audio|Components|Audio|Stop (Variables|Default|GetProjectileRumble))
      (Niagara|SpawnSystematLocation "/Game/RFX/System/FXS_BiggerImpact.FXS_BiggerImpact" _returnvalue)
      (Audio|SpawnSoundatLocation "/Game/Audio/SFX_CoconutBonk.SFX_CoconutBonk" _returnvalue "0, 0, 0" 1.0 1.0 0.5 0 0)
      (Actor|DestroyActor))))

(fn ConstructionScript)