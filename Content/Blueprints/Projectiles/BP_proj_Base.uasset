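; Base projectile Blueprint that supplies impact effects when the actor is destroyed.
; The Destroyed event spawns the pooled, auto-released OnHitFX Niagara system at the ExplosionPos component's location.
; It also plays a random OnHitSounds entry there with randomized pitch, behind a validity check that draws its random pick separately from the playback.
; Movement, collision and damage are not implemented in its graphs.
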(event EventBeginPlay)

(event Collision|EventActorBeginOverlap
  (params (OtherActor :type Actor%20Object%20Reference)))

(event EventTick
  (params (DeltaSeconds :type Float%20%28single-precision%29)))

(event EventDestroyed
  (bind _onhitsounds (Variables|Default|GetonHitSounds))
  (bind _outitem (Utilities|Array|Random _onhitsounds))
  (Niagara|SpawnSystematLocation (Variables|Default|GetonHitFX) (Transformation|GetWorldLocation (Variables|Default|GetExplosionPos)) "0, 0, 0" "1.000000,1.000000,1.000000" true true "AutoRelease")
  (Utilities|IsValid _outitem
    (:Is%20Valid
      (Audio|SpawnSoundatLocation _outitem (Transformation|GetWorldLocation (Variables|Default|GetExplosionPos)) "0, 0, 0" 1.0 (Math|Random|RandomFloatinRange 0.0 1.5) 0.0 0 0))))

(fn ConstructionScript)