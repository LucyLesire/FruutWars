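; Grenade projectile that tumbles at a randomized spin and gets a one-time upward velocity kick on its first tick for a lobbed arc.
; Despawn, destruction, or contact with anything but its owning player triggers Explode, effects, sound, world camera shake and self-destruction.
; The ExplosionRumble component is stopped right after it starts, and a per-player force-feedback loop is left disconnected.
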(event Custom|Rumble
  (Audio|Components|Audio|Play (Variables|Default|GetexplosionRumble) 0.0))

(event Collision|EventActorBeginOverlap
  (params (OtherActor :type Actor%20Object%20Reference))
  (|CallParentFunction OtherActor) ; This node is disabled and will not be called.\nDrag off pins to build functionality.
)

(event EventTick
  (params (DeltaSeconds :type Float%20%28single-precision%29))
  (bind _projectilecomponent (Variables|Default|GetProjectileComponent))
  (|CallParentFunction DeltaSeconds)
  (Utilities|FlowControl|Sequence
    (:then_0
      (Utilities|FlowControl|DoOnce false
        (:Completed
          (Variables|/Script/Engine.MovementComponent|SetVelocity _projectilecomponent (Math|Vector|MakeVector (.x (Variables|/Script/Engine.MovementComponent|GetVelocity _projectilecomponent)) (.y (Variables|/Script/Engine.MovementComponent|GetVelocity _projectilecomponent)) 7.5e+02)))))))

(event EventOnProjectileDespawns
  (bind _returnvalue (Transformation|GetActorLocation))
  (Class|BaseProjectile|Explode)
  (Niagara|SpawnSystematLocation "/Game/RFX/System/FXS_GrenadeApple_explotion.FXS_GrenadeApple_explotion" _returnvalue)
  (Audio|SpawnSoundatLocation "/Game/Audio/SFX_PommeGrenade_Explosion.SFX_PommeGrenade_Explosion" _returnvalue "0, 0, 0" 1.0 1.0 0.0 0 0)
  (CallFunction|Rumble)
  (Audio|Components|Audio|Stop (Variables|Default|GetexplosionRumble))
  (Camera|PlayWorldCameraShake "/Game/Blueprints/Projectiles/BP_ExplosionShake.BP_ExplosionShake_C" (Transformation|GetActorLocation) 0.0 8e+03)
  (Actor|DestroyActor))

(event EventOnProjectileHitCharacter
  (params (target :type Base%20Character%20Object%20Reference))
  (bind _returnvalue (Transformation|GetActorLocation))
  (if (!= (Variables|Default|GetOwningPlayer) target)
    (Class|BaseProjectile|Explode)
    (Niagara|SpawnSystematLocation "/Game/RFX/System/FXS_GrenadeApple_explotion.FXS_GrenadeApple_explotion" _returnvalue)
    (Audio|SpawnSoundatLocation "/Game/Audio/SFX_PommeGrenade_Explosion.SFX_PommeGrenade_Explosion" _returnvalue "0, 0, 0" 1.0 1.0 0.0 0 0)
    (CallFunction|Rumble)
    (Audio|Components|Audio|Stop (Variables|Default|GetexplosionRumble))
    (Camera|PlayWorldCameraShake "/Game/Blueprints/Projectiles/BP_ExplosionShake.BP_ExplosionShake_C" (Transformation|GetActorLocation) 0.0 8e+03)
    (Actor|DestroyActor)))

(event EventProjectileBeginOverlap
  (params (OverlappedComponent :type Primitive%20Component%20Object%20Reference) (OtherActor :type Actor%20Object%20Reference) (OtherComp :type Primitive%20Component%20Object%20Reference) (OtherBodyIndex :type Integer) (bFromSweep :type Boolean) (SweepResult :type Hit%20Result%20Structure%20%28by%20ref%29))
  (bind _returnvalue (Transformation|GetActorLocation))
  (if (!= (Variables|Default|GetOwningPlayer) OtherActor)
    (Class|BaseProjectile|Explode)
    (Niagara|SpawnSystematLocation "/Game/RFX/System/FXS_GrenadeApple_explotion.FXS_GrenadeApple_explotion" _returnvalue)
    (Audio|SpawnSoundatLocation "/Game/Audio/SFX_PommeGrenade_Explosion.SFX_PommeGrenade_Explosion" _returnvalue "0, 0, 0" 1.0 1.0 0.0 0 0)
    (CallFunction|Rumble)
    (Audio|Components|Audio|Stop (Variables|Default|GetexplosionRumble))
    (Camera|PlayWorldCameraShake "/Game/Blueprints/Projectiles/BP_ExplosionShake.BP_ExplosionShake_C" (Transformation|GetActorLocation) 0.0 8e+03)
    (Actor|DestroyActor)))

(event EventDestroyed
  (bind _returnvalue (Transformation|GetActorLocation))
  (Class|BaseProjectile|Explode)
  (Niagara|SpawnSystematLocation "/Game/RFX/System/FXS_GrenadeApple_explotion.FXS_GrenadeApple_explotion" _returnvalue)
  (Audio|SpawnSoundatLocation "/Game/Audio/SFX_PommeGrenade_Explosion.SFX_PommeGrenade_Explosion" _returnvalue "0, 0, 0" 1.0 1.0 0.0 0 0)
  (CallFunction|Rumble)
  (Audio|Components|Audio|Stop (Variables|Default|GetexplosionRumble))
  (Camera|PlayWorldCameraShake "/Game/Blueprints/Projectiles/BP_ExplosionShake.BP_ExplosionShake_C" (Transformation|GetActorLocation) 0.0 8e+03)
  (Actor|DestroyActor))

(event EventBeginPlay
  (bind _returnvalue (Math|Random|RandomFloatinRange -1e+02 1e+02))
  (|CallParentFunction)
  (Variables|/Script/Engine.RotatingMovementComponent|SetRotationRate (Variables|Default|GetRotatingMovement) (Math|Rotator|MakeRotator _returnvalue (Math|Random|RandomFloatinRange -3.5e+02 -2.5e+02) _returnvalue)))

(fn ConstructionScript
  (|CallParentFunction))