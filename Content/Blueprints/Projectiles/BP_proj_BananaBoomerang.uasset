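; Banana boomerang projectile that homes in on nearby players other than its owner.
; On BeginPlay it caches the FW game mode, then each Tick asks it for the closest player within homing range, ignoring the owner's controller.
; A found player's root component becomes the projectile component's homing target, and the rotating movement's spin rate is scaled from the homing acceleration.
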(event EventBeginPlay
  (bind _asfwbase_game_mode (Utilities|Casting|CastToFWBaseGameMode (Game|GetGameMode)))
  (Variables|Default|Setgamemode _asfwbase_game_mode))

(event EventTick
  (params (DeltaSeconds :type Float%20%28single-precision%29))
  (Utilities|IsValid (Variables|Default|GetOwningPlayer)
    (:Is%20Valid
      (bind _asplayer_controller (Utilities|Casting|CastToPlayerController (Pawn|GetController (Variables|Default|GetOwningPlayer))))
      (bind _returnvalue (Class|FWBaseGameMode|GetClosestPlayer (Variables|Default|Getgamemode) (Transformation|GetActorLocation) (Variables|Default|GetHomingRange) _asplayer_controller))
      (Utilities|IsValid _returnvalue
        (:Is%20Valid
          (Variables|/Script/Engine.ProjectileMovementComponent|SetHomingTargetComponent (Variables|Default|GetProjectileComponent) (Variables|/Script/Engine.Actor|GetRootComponent _returnvalue))
          (Variables|/Script/Engine.RotatingMovementComponent|SetRotationRate (Variables|Default|GetRotatingMovement) (Math|Rotator|MakeRotator 0.0 0.0 (* (Variables|/Script/Engine.ProjectileMovementComponent|GetHomingAccelerationMagnitude (Variables|Default|GetProjectileComponent)) 0.1))))))))

(fn ConstructionScript)